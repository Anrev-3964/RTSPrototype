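; Quest pointer actor that periodically traces a navmesh route from the player character to itself.
; A looping timer finds the path synchronously, prints its points for debugging and adds them to the Path spline, which is cleared after a delay matching the timer interval.
; Disconnected leftovers include a second path build and a "Cone Axis" variable update aimed from the pointer toward the player.
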(event `self.ReceiveBeginPlay`
  (`KismetSystemLibrary.K2_SetTimerDelegate` (delegate `Build Nav`) 3.0 true))

(event `Build Nav`
  (bind _path_points (`self.Find Path`))
  (`self.Build Spline` _path_points)
  (`KismetSystemLibrary.Delay` 3.0)
  (`self.Clear Spline`))

(fn `Build Spline`
  (params (`Path points` :type "Array of Vector Structure"))
  (for _array_element `Path points`
    (`SplineComponent.AddSplinePoint` (`self.Path`) _array_element "World" true))
  (return))

(fn `Clear Spline`
  (`SplineComponent.ClearSplinePoints` (`self.Path`) true))

(fn `Find Path`
  (returns (`Path points` :type "Array of Vector Structure"))
  (bind _returnvalue (`NavigationSystemV1.FindPathToActorSynchronously` (`self.K2_GetActorLocation` (`GameplayStatics.GetPlayerCharacter` 0)) self (`self.Tether Distance`) null null))
  (`/Engine/EditorBlueprintResources/StandardMacros.IsValid` _returnvalue
    (:`Is Valid`
      (bind _pathpoints (`NavigationPath.PathPoints` _returnvalue))
      (for _array_element _pathpoints
        (`KismetSystemLibrary.PrintString` (`KismetStringLibrary.Conv_VectorToString` _array_element)))
      (return _pathpoints))))

(fn `UserConstructionScript`)
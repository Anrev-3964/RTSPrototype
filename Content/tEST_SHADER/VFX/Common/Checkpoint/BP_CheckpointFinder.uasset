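; BP_CheckpointFinder is an actor that points a Niagara effect at the BP_Pointer actor nearest the player.
; On BeginPlay it scans all BP_Pointer actors, keeping the closest to the player character within a starting distance threshold.
; It feeds that location to the Niagara "Target Point" variable.
; After a short delay it resets the search state and passes the location to FindCoordinate.
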(event `self.ReceiveBeginPlay`
  (`self.Find Checkpoint`))

(event `Find Checkpoint`
  (bind _output (`|GetArrayItem` (`self.Out Actors`) (`self.ClosestIndex`)))
  (bind _outactors (`GameplayStatics.GetAllActorsOfClass` "/Game/tEST_SHADER/VFX/Common/Checkpoint/BP_Pointer.BP_Pointer_C"))
  (bind _output_get (set `self.Out Actors` _outactors))
  (for (_array_element _array_index) _output_get
    (bind _returnvalue (`KismetMathLibrary.Vector_Distance` (`self.K2_GetActorLocation` (`GameplayStatics.GetPlayerCharacter` 0)) (`self.K2_GetActorLocation` _array_element)))
    (if (> (`self.Distance`) _returnvalue)
      (set `self.Distance` _returnvalue)
      (set `self.ClosestIndex` _array_index)))
  (set `self.Closest Actor` _output)
  (`NiagaraComponent.SetVariableVec3` (`self.Niagara`) "Target Point" (`self.K2_GetActorLocation` _output))
  (`KismetSystemLibrary.Delay` 2.0)
  (`KismetArrayLibrary.Array_Clear` (`self.Out Actors`))
  (set `self.Distance` 20000.0)
  (`self.Find Coordinate` (`self.K2_GetActorLocation` (`self.Closest Actor`))))

(fn `UserConstructionScript`)
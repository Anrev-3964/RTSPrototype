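; Component that finds the nearest checkpoint marker, represented by BP_Pointer actors, and returns its world location.
; FindCheckpoint scans every BP_Pointer in the level, comparing its distance from ThisActor against a stored running minimum to pick ClosestTarget.
; Only when a valid target exists does it reset that minimum to a fixed search range and return the location; ClosestTarget itself is never cleared.
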(fn `Find Checkpoint`
  (returns (`Target Location` :type "Vector Structure"))
  (bind _closest_target (`self.Closest target`))
  (bind _outactors (`GameplayStatics.GetAllActorsOfClass` "/Game/tEST_SHADER/VFX/Common/Checkpoint/BP_Pointer.BP_Pointer_C"))
  (bind _output_get (set `self.Out Actors` _outactors))
  (for _array_element _output_get
    (bind _returnvalue (`KismetMathLibrary.Vector_Distance` (`Actor.K2_GetActorLocation` (`self.ThisActor`)) (`Actor.K2_GetActorLocation` _array_element)))
    (if (> (`self.Distance`) _returnvalue)
      (set `self.Distance` _returnvalue)
      (set `self.Closest target` _array_element)))
  (`/Engine/EditorBlueprintResources/StandardMacros.IsValid` _closest_target
    (:`Is Valid`
      (`KismetArrayLibrary.Array_Clear` (`self.Out Actors`))
      (set `self.Distance` 20000.0)
      (return (`Actor.K2_GetActorLocation` _closest_target)))))